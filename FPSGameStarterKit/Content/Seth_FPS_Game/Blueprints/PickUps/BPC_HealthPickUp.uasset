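; Health pickup that heals the player by HealthToAdd and then destroys itself.
; Use and interact events share a health check: below max it heals, otherwise it calls StoreThisItem to keep the item.
; Overlap by a BP_CharacterBase below max health triggers the same heal, which targets PlayerCast rather than the overlapping actor.
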(event EventBeginPlay
  (|CallParentFunction))

(event Collision|EventActorBeginOverlap
  (params (OtherActor :type Actor%20Object%20Reference))
  (bind _asbp_character_base (Utilities|Casting|CastToBP_CharacterBase OtherActor))
  (if (< (Variables|/Game/Seth_FPS_Game/Blueprints/BP_CharacterBase.BP_CharacterBase_C|GetHealthCurrent _asbp_character_base) (Variables|/Game/Seth_FPS_Game/Blueprints/BP_CharacterBase.BP_CharacterBase_C|GetHealthMax _asbp_character_base))
    (Default|HealthHeal (Variables|Default|GetPlayerCast) (Variables|Default|GetHealthToAdd))
    (Actor|DestroyActor)))

(event EventTick
  (params (DeltaSeconds :type Float%20%28single-precision%29)))

(event EventBPIUseItem
  (bind _playercast (Variables|Default|GetPlayerCast))
  (Math|Float|CompareFloat (Variables|/Game/Seth_FPS_Game/Blueprints/BP_CharacterBase.BP_CharacterBase_C|GetHealthCurrent _playercast) (Variables|/Game/Seth_FPS_Game/Blueprints/BP_CharacterBase.BP_CharacterBase_C|GetHealthMax _playercast)
    (:>
      (CallFunction|StoreThisItem :!label _label))
    (:==
      (goto _label))
    (:<
      (Default|HealthHeal (Variables|Default|GetPlayerCast) (Variables|Default|GetHealthToAdd))
      (Actor|DestroyActor))))

(event EventBPIInteraction
  (bind _playercast (Variables|Default|GetPlayerCast))
  (Math|Float|CompareFloat (Variables|/Game/Seth_FPS_Game/Blueprints/BP_CharacterBase.BP_CharacterBase_C|GetHealthCurrent _playercast) (Variables|/Game/Seth_FPS_Game/Blueprints/BP_CharacterBase.BP_CharacterBase_C|GetHealthMax _playercast)
    (:>
      (CallFunction|StoreThisItem :!label _label))
    (:==
      (goto _label))
    (:<
      (Default|HealthHeal (Variables|Default|GetPlayerCast) (Variables|Default|GetHealthToAdd))
      (Actor|DestroyActor))))

(fn ConstructionScript)